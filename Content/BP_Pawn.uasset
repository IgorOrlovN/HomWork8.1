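; Player pawn that moves along the world X axis and puts a ball into play, apparently as a paddle.
; On BeginPlay, SpawnBall spawns a scaled-down BP_Ball at the capsule's location, stores it as PlaingBall and binds to its OnDead event.
; Two handlers of the move axis apply a swept, fixed-step world offset in the input's direction, without delta-time scaling.
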(event `self.ReceiveBeginPlay`
  (`self.SpawnBall`))

(event `InputAxis|move`
  (params (AxisValue :type "Float (single-precision)"))
  (if (< AxisValue 0.0)
    (`self.K2_AddActorWorldOffset` (-10.0 0.0 0.0) true)))

(event `InputAxis|move`
  (params (AxisValue :type "Float (single-precision)"))
  (if (> AxisValue 0.0)
    (`self.K2_AddActorWorldOffset` (10.0 0.0 0.0) true)))

(fn `SpawnBall`
  (bind _returnvalue (`|SpawnActorFromClass` "/Game/BP_Ball.BP_Ball_C" (`KismetMathLibrary.MakeTransform` (`SceneComponent.K2_GetComponentLocation` (`self.Capsule`)) (struct) (0.3 0.3 0.3)) "AlwaysSpawn" "OverrideRootScale" null null))
  (bind _output_get (set `self.PlaingBall` _returnvalue))
  (add `/Game/BP_Ball.OnDead` _output_get (`|CreateDelegate` :!event `SpawnBall`))
  (return))

(fn `UserConstructionScript`)