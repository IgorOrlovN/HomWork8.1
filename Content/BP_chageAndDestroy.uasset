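; BP_chageAndDestroy is a block actor that takes hits from BP_Ball, changing appearance and then breaking.
; Its Hit event ignores other actors and checks a Hit counter.
; While the counter is at least one, a hit switches the Cube to a clay brick material and decrements it.
; Once it drops below one, the next hit destroys the actor, usually spawning a BP_SpawnCube at the Cube's location first.
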(event `self.ReceiveActorBeginOverlap`
  (params (OtherActor :type "Actor Object Reference")))

(event `self.ReceiveHit`
  (params (MyComp :type "PrimitiveComponent Object Reference") (Other :type "Actor Object Reference") (OtherComp :type "PrimitiveComponent Object Reference") (bSelfMoved :type Boolean) (HitLocation :type "Vector Structure") (HitNormal :type "Vector Structure") (NormalImpulse :type "Vector Structure") (Hit :type "HitResult Structure (by ref)"))
  (cast `/Game/BP_Ball` Other)
  (if (< (`self.hit`) 1.0)
    (if (< (`KismetMathLibrary.RandomInteger` 100) 90)
      (`|SpawnActorFromClass` "/Game/BP_SpawnCube.BP_SpawnCube_C" (`KismetMathLibrary.MakeTransform` (`SceneComponent.K2_GetComponentLocation` (`self.Cube`))) "AlwaysSpawn" "OverrideRootScale" null null))
    (`self.K2_DestroyActor`)
    (else
      (`PrimitiveComponent.SetMaterial` (`self.Cube`) 0 "/Game/StarterContent/Materials/M_Brick_Clay_New.M_Brick_Clay_New")
      (`/Engine/EditorBlueprintResources/StandardMacros.DecrementFloat` (`self.hit`)))))

(fn `UserConstructionScript`)